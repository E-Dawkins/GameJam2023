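; Enemy AI Blueprint that waits out a countdown, then chases the player and restarts the current level on reaching them.
; BeginPlay seeds the countdown from TimeForEnemyToAttack and adds a Timer widget to the viewport.
; Tick uses a one-second Delay to decrement Seconds, then calls FollowPlayer at zero.
; FollowPlayer runs AIMoveTo toward the player character and reopens the level by name on success.
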(event Custom|FollowPlayer
  (if (Variables|Default|GetTimerDone)
    (AI|AIMoveTo self "0, 0, 0" (Game|GetPlayerCharacter 0) 5.0 false
      (:OnSuccess
        (bind _returnvalue (Game|GetCurrentLevelName true))
        (Game|OpenLevel(byName) (Utilities|String|StringToName _returnvalue))))))

(event EventBeginPlay
  (Variables|Default|SetSeconds (Variables|Default|GetTimeForEnemyToAttack))
  (bind _returnvalue (UserInterface|CreateWidget "/Game/Scenes/JustinScripts/Timer.Timer_C"))
  (UserInterface|Viewport|AddtoViewport _returnvalue 0))

(event EventTick
  (params (DeltaSeconds :type Float%20%28single-precision%29))
  (if (not (Variables|Default|GetTimerDone))
    (Utilities|FlowControl|Delay 1.0)
    (bind _output_get (Variables|Default|SetSeconds (- (Variables|Default|GetSeconds) 1)))
    (if (<= _output_get 0)
      (Variables|Default|SetTimerDone true)
      (CallFunction|FollowPlayer))))

(fn ConstructionScript)